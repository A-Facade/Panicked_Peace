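; Gun pickup that the player character steals once on overlapping its box, alerting a soldier.
; The first overlap calls StolenGun on Bp_Chara, switches the SoldierIdle flipbook to walking and plays an alert sound.
; After a short delay it replays the alert, destroys itself, then attempts to spawn a Bp_Enemey_V2 AI at its location through a cast of a variable.
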(event OnComponentBeginOverlap(Box)
  (params (OverlappedComponent :type Primitive%20Component%20Object%20Reference) (OtherActor :type Actor%20Object%20Reference) (OtherComp :type Primitive%20Component%20Object%20Reference) (OtherBodyIndex :type Integer) (bFromSweep :type Boolean) (SweepResult :type Hit%20Result%20Structure%20%28by%20ref%29))
  (if (not (Variables|Default|GetTouched%20Once))
    (Variables|Default|SetTouched%20Once true)
    (bind _asbp_chara (Utilities|Casting|CastToBp_Chara OtherActor))
    (Default|StolenGun _asbp_chara)
    (Sprite|SetFlipbook (Variables|Default|GetSoldier_Idle) "/Game/Lesson/Sprites/Mine/Soldier/Soldier_Walk.Soldier_Walk")
    (Audio|PlaySound2D "/Game/Lesson/Sounds/Cues/Sc_SoldierAlert.Sc_SoldierAlert")
    (Utilities|FlowControl|Delay 1.0)
    (Audio|PlaySound2D "/Game/Lesson/Sounds/Cues/Sc_SoldierAlert.Sc_SoldierAlert")
    (Actor|DestroyActor)
    (bind _asbp_enemey_v2 (Utilities|Casting|CastToBp_Enemey_V2Class "/Game/Lesson/Blueprints/Bp_Enemey_V2.Bp_Enemey_V2_C"))
    (AI|SpawnAIFromClass _asbp_enemey_v2 0 (Transformation|GetActorLocation) "0, 0, 0" false)))

(event EventBeginPlay)

(event Collision|EventActorBeginOverlap
  (params (OtherActor :type Actor%20Object%20Reference)))

(event EventTick
  (params (DeltaSeconds :type Float%20%28single-precision%29)))

(fn ConstructionScript)