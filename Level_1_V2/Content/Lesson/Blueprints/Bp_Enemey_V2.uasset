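; Side-scrolling flipbook soldier enemy that chases Bp_Chara along X while the player is inside its detection sphere.
; Tick drives that chase, picks animations from movement state and flips rotation to face travel.
; Overlapped zone actors set the surface used for landing sounds and frame-timed footsteps.
; Move and jump input handlers are also present, box-overlap damage is disconnected, and StolenGun increments the player's gun counter with debug prints.
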(event OnComponentBeginOverlap(Sphere)
  (params (OverlappedComponent :type Primitive%20Component%20Object%20Reference) (OtherActor :type Actor%20Object%20Reference) (OtherComp :type Primitive%20Component%20Object%20Reference) (OtherBodyIndex :type Integer) (bFromSweep :type Boolean) (SweepResult :type Hit%20Result%20Structure%20%28by%20ref%29))
  ;[1 1 1] Player Detection
  (Utilities|Casting|CastToBp_Chara OtherActor)
  (Variables|Default|SetIsOverlapping true))

(event OnComponentEndOverlap(Sphere)
  (params (OverlappedComponent :type Primitive%20Component%20Object%20Reference) (OtherActor :type Actor%20Object%20Reference) (OtherComp :type Primitive%20Component%20Object%20Reference) (OtherBodyIndex :type Integer))
  ;[1 1 1] Player Detection
  (Utilities|Casting|CastToBp_Chara OtherActor)
  (Variables|Default|SetIsOverlapping false))

(event OnComponentBeginOverlap(Box)
  (params (OverlappedComponent :type Primitive%20Component%20Object%20Reference) (OtherActor :type Actor%20Object%20Reference) (OtherComp :type Primitive%20Component%20Object%20Reference) (OtherBodyIndex :type Integer) (bFromSweep :type Boolean) (SweepResult :type Hit%20Result%20Structure%20%28by%20ref%29)))

(event Custom|UpdateAnimation
  ;[1 1 1] Handle Animation
  (switch Utilities|FlowControl|Switch|SwitchonBp_States (Variables|Default|GetState)
    (:NewEnumerator0
      (if (> (Math|Vector|VectorLength (Transformation|GetVelocity)) 0.0)
        (Sprite|SetFlipbook (Variables|Default|GetSprite) "/Game/Lesson/Sprites/Mine/Soldier/Soldier_Walk.Soldier_Walk")
        (else
          (Sprite|SetFlipbook (Variables|Default|GetSprite) "/Game/Lesson/Sprites/Mine/Soldier/Soldier_Idle.Soldier_Idle"))))
    (:NewEnumerator2
      (Sprite|SetFlipbook (Variables|Default|GetSprite) "/Game/Lesson/Sprites/Mine/Soldier/Soldier_Jump.Soldier_Jump"))))

(event EventTick
  (params (DeltaSeconds :type Float%20%28single-precision%29))
  ;[1 1 1] Tick - Updates animation
  (Utilities|FlowControl|Sequence
    (:then_0
      ;[1 1 1] Handle Animation
      (if (Variables|Default|GetIsOverlapping)
        (bind _asbp_chara (Utilities|Casting|CastToBp_Chara (Game|GetPlayerCharacter 0)))
        (if (>= (- (.x (Transformation|GetWorldLocation (Variables|/Script/Engine.Character|GetCapsuleComponent _asbp_chara))) (.x (Transformation|GetWorldLocation (Variables|Collision|GetCapsuleComponent)))) 0.0)
          (Variables|Default|SetisMovingRight true)
          (else
            (Variables|Default|SetisMovingRight false)))
        (Pawn|Input|AddMovementInput "1.000000, 0, 0" (- (.x (Transformation|GetWorldLocation (Variables|/Script/Engine.Character|GetCapsuleComponent _asbp_chara))) (.x (Transformation|GetWorldLocation (Variables|Collision|GetCapsuleComponent)))) false)))
    (:then_1
      (CallFunction|UpdateAnimation)
      (Math|Float|CompareFloat (.X (Math|Vector|BreakVector (Variables|/Script/Engine.MovementComponent|GetVelocity (Pawn|GetMovementComponent)))) 0.0
        (:>
          (Transformation|SetActorRotation (Math|Rotator|MakeRotator 0.0 0.0 0.0) :!label _label))
        (:==
          (if (Variables|Default|GetisMovingRight)
            (goto _label)
            (else
              (Transformation|SetActorRotation (Math|Rotator|MakeRotator 0.0 0.0 1.8e+02) :!label _label_2))))
        (:<
          (goto _label_2)))
      ;[1 1 1] Footstep Sounds
      (if (or (== (Class|PaperFlipbookComponent|GetPlaybackPositioninFrames (Variables|Default|GetSprite)) 3) (== 0 7))
        (if (> (Math|Vector|VectorLength (Transformation|GetVelocity)) 0.0)
          (if (AI|Components|NavMovement|IsMovingonGround (Variables|Character|GetCharacterMovement))
            (CallFunction|FootstepsSounds)))))))

(event EventOnLanded
  (params (Hit :type Hit%20Result%20Structure%20%28by%20ref%29))
  ;[1 1 1] Handle Jump
  (Variables|Default|SetState "NewEnumerator0")
  (CallFunction|LandingSounds))

(event Collision|EventActorBeginOverlap
  (params (OtherActor :type Actor%20Object%20Reference))
  ;[1 1 1] Detect Colision
  (Utilities|FlowControl|Sequence
    (:then_4
      ;[1 1 1] Sound Type Zones
      (Utilities|Casting|CastToBp_ZoneMetal OtherActor)
      (Variables|Default|SetZone "Metal"))
    (:then_5
      (Utilities|Casting|CastToBp_ZoneRaft OtherActor)
      (Variables|Default|SetZone "Raft"))
    (:then_6
      (Utilities|Casting|CastToBp_ZoneRock OtherActor)
      (Variables|Default|SetZone "Rock"))
    (:then_7
      (Utilities|Casting|CastToBp_ZoneSand OtherActor)
      (Variables|Default|SetZone "Sand"))
    (:then_8
      (Utilities|Casting|CastToBp_ZoneWood OtherActor)
      (Variables|Default|SetZone "Wood"))))

(event Input|ActionEvents|InputActionJump
  (params (Key :type Key%20Structure))
  ;[1 1 1] Handle Jump
  (:Pressed
    (Character|Jump)
    (if (not (AI|Components|NavMovement|IsFalling (Variables|Character|GetCharacterMovement)))
      (Audio|PlaySound2D "/Game/Lesson/Sounds/Cues/Sc_Jump.Sc_Jump")
      (Variables|Default|SetState "NewEnumerator2")))
  (:Released
    (Character|StopJumping)))

(event Input|AxisEvents|InputAxisMoveRight
  (params (AxisValue :type Float%20%28single-precision%29))
  ;[1 1 1] Handle movement
  (if (> AxisValue 0.0)
    (Variables|Default|SetisMovingRight true)
    (elif (< AxisValue 0.0)
      (Variables|Default|SetisMovingRight false)))
  (Pawn|Input|AddMovementInput "1.000000, 0, 0" AxisValue false))

(event Input|TouchEvents|InputTouch
  (params (Location :type Vector) (FingerIndex :type ETouchIndex%20Enum))
  ;[1 1 1] Handle Jump
  (:Released
    (Character|StopJumping)))

(fn ConstructionScript)

(fn StolenGun
  (bind _asbp_chara (Utilities|Casting|CastToBp_Chara (Game|GetPlayerCharacter 0)))
  (bind _result (Math|Integer|IncrementInt (Variables|/Game/Lesson/Blueprints/Bp_Chara.Bp_Chara_C|GetSGun _asbp_chara))
    (:%20%20
      (bind _output_get (Variables|Default|SetSGun _result))
      (Development|PrintString "GUNS")
      (Development|PrintString (Utilities|String|ToString(Integer) _output_get)))))

(fn FootstepsSounds
  (bind _zone (Variables|Default|GetZone))
  (if (Utilities|Enum|Equal(Enum) _zone "Metal")
    (Audio|PlaySound2D "/Game/Lesson/Sounds/Cues/Sc_MetalWalk.Sc_MetalWalk")
    (elif (Utilities|Enum|Equal(Enum) _zone "Raft")
      (Audio|PlaySound2D "/Game/Lesson/Sounds/Cues/Sc_RaftWalk.Sc_RaftWalk")
      (elif (Utilities|Enum|Equal(Enum) _zone "Wood")
        (Audio|PlaySound2D "/Game/Lesson/Sounds/Cues/Sc_WoodWalk.Sc_WoodWalk")
        (elif (Utilities|Enum|Equal(Enum) _zone "Sand")
          (Audio|PlaySound2D "/Game/Lesson/Sounds/Cues/Sc_SandWalk.Sc_SandWalk")
          (elif (Utilities|Enum|Equal(Enum) _zone "Rock")
            (Audio|PlaySound2D "/Game/Lesson/Sounds/Cues/Sc_RockWalk.Sc_RockWalk")))))))

(fn LandingSounds
  (bind _zone (Variables|Default|GetZone))
  (if (Utilities|Enum|Equal(Enum) _zone "Metal")
    (Audio|PlaySound2D "/Game/Lesson/Sounds/Cues/Sc_MetalLand.Sc_MetalLand")
    (elif (Utilities|Enum|Equal(Enum) _zone "Raft")
      (Audio|PlaySound2D "/Game/Lesson/Sounds/Cues/Sc_RaftLand.Sc_RaftLand")
      (elif (Utilities|Enum|Equal(Enum) _zone "Wood")
        (Audio|PlaySound2D "/Game/Lesson/Sounds/Cues/Sc_WoodLand.Sc_WoodLand")
        (elif (Utilities|Enum|Equal(Enum) _zone "Sand")
          (Audio|PlaySound2D "/Game/Lesson/Sounds/Cues/Sc_SandLand.Sc_SandLand")
          (elif (Utilities|Enum|Equal(Enum) _zone "Rock")
            (Audio|PlaySound2D "/Game/Lesson/Sounds/Cues/Sc_RockLand.Sc_RockLand")))))))