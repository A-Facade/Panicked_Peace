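; Player character for a 2D Paper2D side-scroller, with walking, jumping, left and right launch dashes, and bullet shooting.
; Tick drives flipbook selection from a State enum, flips facing via controller yaw, and triggers footsteps on a walk frame.
; Overlap casts handle hazard damage, health pickups, checkpoints, end-of-level teleport, and surface zones that select footstep and landing sounds.
; Depleted health sets Dead, disabling input and showing GameOver.
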(event Custom|UpdateAnimation
  (bind _returnvalue (Game|GetPlayerController 0))
  ;[1 1 1] Handle Animation
  (Utilities|FlowControl|Sequence
    (:then_0
      (switch Utilities|FlowControl|Switch|SwitchonBp_States (Variables|Default|GetState)
        (:NewEnumerator0
          (if (> (Math|Vector|VectorLength (Transformation|GetVelocity)) 0.0)
            (Sprite|SetFlipbook (Variables|Default|GetSprite) "/Game/Lesson/Sprites/Mine/Hippie/Hippie_Walking.Hippie_Walking")
            (else
              (Sprite|SetFlipbook (Variables|Default|GetSprite) "/Game/Lesson/Sprites/Mine/Hippie/Hippie_IDLE+BLINK.Hippie_IDLE+BLINK"))))
        (:NewEnumerator2
          (Sprite|SetFlipbook (Variables|Default|GetSprite) "/Game/Lesson/Sprites/Mine/Hippie/Hippie_Jumping.Hippie_Jumping"))
        (:NewEnumerator4
          (Sprite|SetFlipbook (Variables|Default|GetSprite) "/Game/Lesson/Sprites/Mine/Hippie/Hippie_Dead.Hippie_Dead")
          (Input|DisableInput (Game|GetPlayerCharacter 0) _returnvalue)
          (Utilities|FlowControl|Delay 0.5)
          (bind _returnvalue_2 (UserInterface|CreateWidget "/Game/Lesson/Menus/GameOver.GameOver_C"))
          (UserInterface|Viewport|AddtoViewport _returnvalue_2 0)
          (Variables|/Script/Engine.PlayerController|SetbShowMouseCursor _returnvalue true))
        (:NewEnumerator3
          (Variables|Default|SetIsDashing true)
          (Sprite|SetFlipbook (Variables|Default|GetSprite) "/Game/Lesson/Sprites/Mine/Hippie/Hippie_Dash1.Hippie_Dash1")
          (Utilities|FlowControl|Delay 0.25)
          (Variables|Default|SetState "NewEnumerator8"))
        (:NewEnumerator8
          (Sprite|SetFlipbook (Variables|Default|GetSprite) "/Game/Lesson/Sprites/Mine/Hippie/Hippie_Dash2.Hippie_Dash2"))
        (:NewEnumerator9
          ;;[1 1 1] Dash 3 Animation (Error)
          (Sprite|SetFlipbook (Variables|Default|GetSprite) "/Game/Lesson/Sprites/Mine/Hippie/Hippie_Dash3.Hippie_Dash3")
          (CallFunction|LandingSounds)
          (Utilities|FlowControl|Delay 1e+01)
          (Variables|Default|SetIsDashing false)
          (Variables|Default|SetState "NewEnumerator0"))))
    (:then_1
      (if (not (Math|Boolean|Equal(Boolean) (Variables|Default|GetIsDashing) true))
        (Variables|Default|SetState "NewEnumerator0")))))

(event Custom|Check%20For%20Death
  ;[1 1 1] Health System
  (if (<= (stale Collision|EventActorBeginOverlap _output_get) 0.0)
    (Variables|Default|SetState "NewEnumerator4")
    (else
      (Audio|PlaySound2D "/Game/Lesson/Sounds/Cues/Sc_PlayerHurt.Sc_PlayerHurt"))))

(event EventTick
  (params (DeltaSeconds :type Float%20%28single-precision%29))
  ;[1 1 1] Tick - Updates animation
  (CallFunction|UpdateAnimation)
  (Math|Float|CompareFloat (.X (Math|Vector|BreakVector (Variables|/Script/Engine.MovementComponent|GetVelocity (Pawn|GetMovementComponent)))) 0.0
    (:>
      (Pawn|SetControlRotation (Pawn|GetController) (Math|Rotator|MakeRotator 0.0 0.0 0.0) :!label _label))
    (:==
      (if (Variables|Default|GetisMovingRight)
        (goto _label)
        (else
          (Pawn|SetControlRotation (Pawn|GetController) (Math|Rotator|MakeRotator 0.0 0.0 1.8e+02) :!label _label_2))))
    (:<
      (goto _label_2)))
  ;[1 1 1] Footstep Sounds
  (if (or (== (Class|PaperFlipbookComponent|GetPlaybackPositioninFrames (Variables|Default|GetSprite)) 3) (== 0 7))
    (if (> (Math|Vector|VectorLength (Transformation|GetVelocity)) 0.0)
      (if (AI|Components|NavMovement|IsMovingonGround (Variables|Character|GetCharacterMovement))
        (CallFunction|FootstepsSounds)))))

(event EventOnLanded
  (params (Hit :type Hit%20Result%20Structure%20%28by%20ref%29))
  ;[1 1 1] Handle Jump
  (Variables|Default|SetIsDashing false)
  (Variables|Default|SetState "NewEnumerator0")
  (CallFunction|LandingSounds))

(event EventBeginPlay
  ;[1 1 1] Main Menu Set Up
  (Utilities|FlowControl|Sequence
    (:then_0
      (Class|ActorComponent|SetIsReplicated (Variables|Default|GetSprite) true))
    (:then_1
      (Audio|PlaySound2D "/Game/Lesson/Sounds/Cues/Sc_Sea.Sc_Sea")
      (Audio|PlaySound2D "/Game/Lesson/Sounds/Cues/Sc_Seagull.Sc_Seagull"))
    (:then_2
      (Class|PlayerController|SetAudioListenerOverride (Game|GetPlayerController 0) (Variables|Collision|GetCapsuleComponent) "0, 0, 0" "0, 0, 0"))))

(event Collision|EventActorBeginOverlap
  (params (OtherActor :type Actor%20Object%20Reference))
  ;[1 1 1] Detect Colision
  (Utilities|FlowControl|Sequence
    (:then_0
      ;[1 1 1] Health System
      (Utilities|Casting|CastToBp_DamageSpike OtherActor)
      (bind _output_get (Variables|Default|SetHealthCurrent (- (Variables|Default|GetHealthCurrent) 0.25) :!label _label))
      (if (<= _output_get 0.0) :!label _label_2
        (Variables|Default|SetState "NewEnumerator4")
        (else
          (Audio|PlaySound2D "/Game/Lesson/Sounds/Cues/Sc_PlayerHurt.Sc_PlayerHurt"))))
    (:then_1
      ;[1 1 1] Health Pickup
      (bind _asbp_health_pickup (Utilities|Casting|CastToBp_HealthPickup OtherActor))
      (Variables|Default|SetHealthCurrent (+ (Variables|Default|GetHealthCurrent) 1.0))
      (Actor|DestroyActor _asbp_health_pickup))
    (:then_2
      (Utilities|Casting|CastToBp_FanBlade OtherActor)
      (Variables|Default|SetHealthCurrent (- (Variables|Default|GetHealthCurrent) 0.34))
      (goto _label_2))
    (:then_3
      (Utilities|Casting|CastToBp_Void OtherActor)
      (goto _label))
    (:then_4
      ;[1 1 1] Sound Type Zones
      (Utilities|Casting|CastToBp_ZoneMetal OtherActor)
      (Variables|Default|SetZone "Metal"))
    (:then_5
      (Utilities|Casting|CastToBp_ZoneRaft OtherActor)
      (Variables|Default|SetZone "Raft"))
    (:then_6
      (Utilities|Casting|CastToBp_ZoneRock OtherActor)
      (Variables|Default|SetZone "Rock"))
    (:then_7
      (Utilities|Casting|CastToBp_ZoneSand OtherActor)
      (Variables|Default|SetZone "Sand"))
    (:then_8
      (Utilities|Casting|CastToBp_ZoneWood OtherActor)
      (Variables|Default|SetZone "Wood"))
    (:then_9
      ;[1 1 1] End Level Detection
      (Utilities|Casting|CastToBp_EndLevel OtherActor)
      (Transformation|Teleport "5356.000000, 0,1136.000000" "0, 0, 0")
      (Audio|PlaySound2D "/Game/Lesson/Sounds/Cues/Sc_EndOfLevel.Sc_EndOfLevel"))
    (:then_10
      ;[1 1 1] Simple Checkpoint
      (Utilities|Casting|CastToBp_Checkpoint OtherActor)
      (Variables|Default|SetPassedCheckpoint true)
      (Audio|PlaySound2D "/Game/Lesson/Sounds/Cues/Sc_Checkpoint.Sc_Checkpoint"))))

(event Input|ActionEvents|InputActionJump
  (params (Key :type Key%20Structure))
  ;[1 1 1] Handle Jump
  (:Pressed
    (Character|Jump)
    (if (not (AI|Components|NavMovement|IsFalling (Variables|Character|GetCharacterMovement)))
      (Audio|PlaySound2D "/Game/Lesson/Sounds/Cues/Sc_Jump.Sc_Jump")
      (Variables|Default|SetState "NewEnumerator2")))
  (:Released
    (Character|StopJumping)))

(event Input|AxisEvents|InputAxisMoveRight
  (params (AxisValue :type Float%20%28single-precision%29))
  ;[1 1 1] Handle movement
  (if (> AxisValue 0.0)
    (Variables|Default|SetisMovingRight true)
    (elif (< AxisValue 0.0)
      (Variables|Default|SetisMovingRight false)))
  (Pawn|Input|AddMovementInput "1.000000, 0, 0" AxisValue false))

(event Input|KeyboardEvents|Q
  (params (Key :type Key%20Structure))
  ;[1 1 1] Left Dash
  (:Pressed
    (Character|LaunchCharacter (Math|Vector|MakeVector -3e+02 0.0 2e+02) false false)
    (Variables|Default|SetState "NewEnumerator3")))

(event Input|KeyboardEvents|E
  (params (Key :type Key%20Structure))
  ;[1 1 1] Right Dash
  (:Pressed
    (Character|LaunchCharacter (Math|Vector|MakeVector 3e+02 0.0 2e+02) false false)
    (Variables|Default|SetState "NewEnumerator3")))

(event Input|MouseEvents|LeftMouseButton
  (params (Key :type Key%20Structure))
  ;[1 1 1] Shooting
  (:Pressed
    (Variables|Default|SetState "NewEnumerator6")
    (Game|SpawnActorfromClass "/Game/Lesson/Blueprints/Bp_Bullet.Bp_Bullet_C" (Transformation|GetWorldTransform (Variables|Default|GetShooting%20Arrow)) "Undefined" 0 0))
  (:Released
    (Variables|Default|SetState "NewEnumerator0")))

(event Input|TouchEvents|InputTouch
  (params (Location :type Vector) (FingerIndex :type ETouchIndex%20Enum))
  ;[1 1 1] Handle Jump
  (:Released
    (Character|StopJumping)))

(fn ConstructionScript)

(fn StolenGun
  (bind _asbp_chara (Utilities|Casting|CastToBp_Chara (Game|GetPlayerCharacter 0)))
  (bind _result (Math|Integer|IncrementInt (Variables|Bp_Chara_C|GetSGun _asbp_chara))
    (:%20%20
      (bind _output_get (Variables|Default|SetSGun _result))
      (Development|PrintString "GUNS")
      (Development|PrintString (Utilities|String|ToString(Integer) _output_get)))))

(fn FootstepsSounds
  (bind _zone (Variables|Default|GetZone))
  (if (Utilities|Enum|Equal(Enum) _zone "Metal")
    (Audio|PlaySound2D "/Game/Lesson/Sounds/Cues/Sc_MetalWalk.Sc_MetalWalk")
    (elif (Utilities|Enum|Equal(Enum) _zone "Raft")
      (Audio|PlaySound2D "/Game/Lesson/Sounds/Cues/Sc_RaftWalk.Sc_RaftWalk")
      (elif (Utilities|Enum|Equal(Enum) _zone "Wood")
        (Audio|PlaySound2D "/Game/Lesson/Sounds/Cues/Sc_WoodWalk.Sc_WoodWalk")
        (elif (Utilities|Enum|Equal(Enum) _zone "Sand")
          (Audio|PlaySound2D "/Game/Lesson/Sounds/Cues/Sc_SandWalk.Sc_SandWalk")
          (elif (Utilities|Enum|Equal(Enum) _zone "Rock")
            (Audio|PlaySound2D "/Game/Lesson/Sounds/Cues/Sc_RockWalk.Sc_RockWalk")))))))

(fn LandingSounds
  (bind _zone (Variables|Default|GetZone))
  (if (Utilities|Enum|Equal(Enum) _zone "Metal")
    (Audio|PlaySound2D "/Game/Lesson/Sounds/Cues/Sc_MetalLand.Sc_MetalLand")
    (elif (Utilities|Enum|Equal(Enum) _zone "Raft")
      (Audio|PlaySound2D "/Game/Lesson/Sounds/Cues/Sc_RaftLand.Sc_RaftLand")
      (elif (Utilities|Enum|Equal(Enum) _zone "Wood")
        (Audio|PlaySound2D "/Game/Lesson/Sounds/Cues/Sc_WoodLand.Sc_WoodLand")
        (elif (Utilities|Enum|Equal(Enum) _zone "Sand")
          (Audio|PlaySound2D "/Game/Lesson/Sounds/Cues/Sc_SandLand.Sc_SandLand")
          (elif (Utilities|Enum|Equal(Enum) _zone "Rock")
            (Audio|PlaySound2D "/Game/Lesson/Sounds/Cues/Sc_RockLand.Sc_RockLand")))))))