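; Bp_Checker is a checkpoint actor that only clears when the player character's SGun value is above zero.
; Every tick it reads SGun from the player's Bp_Chara and switches its flipbook between locked and unlocked.
; When Bp_Chara overlaps its box, it either plays a deny sound or plays an allow sound and destroys itself, printing No or Yes.
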(event OnComponentBeginOverlap(Box)
  (params (OverlappedComponent :type Primitive%20Component%20Object%20Reference) (OtherActor :type Actor%20Object%20Reference) (OtherComp :type Primitive%20Component%20Object%20Reference) (OtherBodyIndex :type Integer) (bFromSweep :type Boolean) (SweepResult :type Hit%20Result%20Structure%20%28by%20ref%29))
  ;[1 1 1] Player Colision
  (bind _asbp_chara (Utilities|Casting|CastToBp_Chara OtherActor))
  (if (<= (Variables|/Game/Lesson/Blueprints/Bp_Chara.Bp_Chara_C|GetSGun _asbp_chara) 0)
    ;[1 1 1] Play Sound
    (Audio|PlaySound2D "/Game/Lesson/Sounds/Cues/Sc_CheckerDeny_Cue.Sc_CheckerDeny_Cue")
    (Development|PrintString "No")
    (else
      (Audio|PlaySound2D "/Game/Lesson/Sounds/Cues/Sc_CheckerAllow_Cue.Sc_CheckerAllow_Cue")
      (Actor|DestroyActor)
      (Development|PrintString "Yes"))))

(event Collision|EventActorBeginOverlap
  (params (OtherActor :type Actor%20Object%20Reference)))

(event EventTick
  (params (DeltaSeconds :type Float%20%28single-precision%29))
  (bind _paperflipbook (Variables|Default|GetPaperFlipbook))
  ;[1 1 1] Update Animation Error
  (bind _asbp_chara (Utilities|Casting|CastToBp_Chara (Game|Player|GetPlayerPawn 0)))
  (if (<= (Variables|/Game/Lesson/Blueprints/Bp_Chara.Bp_Chara_C|GetSGun _asbp_chara) 0)
    (Sprite|SetFlipbook _paperflipbook "/Game/Lesson/Sprites/Mine/Checker_Locked.Checker_Locked")
    (else
      (Sprite|SetFlipbook _paperflipbook "/Game/Lesson/Sprites/Mine/Checker_Unlocked.Checker_Unlocked"))))

(fn ConstructionScript)